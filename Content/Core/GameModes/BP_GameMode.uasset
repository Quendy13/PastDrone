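; Game mode that runs a countdown and triggers the player's lose condition when time runs out.
; On BeginPlay it caches the first-person character and starts a looping one-second timer.
; Each tick of that timer decrements Time, pushes it to the character's HUD and calls Loose on the character at zero or below.
; The timer is never cleared here, so it keeps firing after expiry.
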(event Custom|StartTimer
  (Utilities|Time|SetTimerbyEvent (delegate Custom|Timer) 1.0 true))

(event Custom|Timer
  (bind _result (Math|Float|DecrementFloat (Variables|Default|GetTime))
    (:%20%20
      (Default|TimerUpdate (Variables|/Game/FirstPerson/Blueprints/BP_FirstPersonCharacter.BP_FirstPersonCharacter_C|GetHUDRef (Variables|Default|GetCharacterRf)) _result)
      (if (<= _result 0.0)
        (Default|Loose (Variables|Default|GetCharacterRf))))))

(event EventBeginPlay
  (bind _asbp_first_person_character (Utilities|Casting|CastToBP_FirstPersonCharacter (Game|GetPlayerCharacter 0)))
  (Variables|Default|SetCharacterRf _asbp_first_person_character)
  (CallFunction|StartTimer))

(fn ConstructionScript)